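; A generated dynamic mesh Blueprint that tessellates and displaces a static mesh using Geometry Script.
; On rebuild, unless frozen, it resets the dynamic mesh, copies in the source static mesh and applies PN tessellation at the set subdivision level.
; If a height map is valid, it displaces the result by that texture and recomputes normals.
; The bake-to-static-mesh function is an empty stub.
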(event `self.OnRebuildGeneratedMesh`
  (params (TargetMesh :type "DynamicMesh Object Reference"))
  (if (not (`self.isFrozen`))
    (bind _returnvalue (`DynamicMesh.Reset` TargetMesh))
    (bind _target_mesh (`self.Target-Mesh`)
      (:`then`
        (bind _returnvalue_2 (`GeometryScriptLibrary_StaticMeshFunctions.CopyMeshFromStaticMesh` _target_mesh _returnvalue (struct) (struct) null)
          (:`Success`
            (bind _returnvalue_3 (`GeometryScriptLibrary_MeshSubdivideFunctions.ApplyPNTessellation` _returnvalue_2 (struct) (`self.Subdivisions`) null))
            (bind _height_map (`self.Height-Map`)
              (:`then`
                (bind _returnvalue_4 (`GeometryScriptLibrary_MeshDeformFunctions.ApplyDisplaceFromTextureMap` _returnvalue_3 _height_map (make `GeometryScriptDisplaceFromTextureOptions` (`self.Displacement-Amount`)) 0 null))
                (`GeometryScriptLibrary_MeshNormalsFunctions.RecomputeNormals` _returnvalue_4 (struct) null))
              (:`else`)))))
      (:`else`))))

(fn `Bake-To-Static-Mesh`)

(fn `UserConstructionScript`)